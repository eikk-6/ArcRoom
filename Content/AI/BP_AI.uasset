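; BP_AI is a zombie monster that senses the player, plays chase music and makes melee attacks.
; PawnSensing sets the seeingPlayer blackboard key and fades in chase music on sighting a Player-tagged pawn.
; A looping timer clears that key, then fades the music out if it stays false after a delay.
; AttackPlayer plays a montage, immediately sphere-traces forward to apply damage, and blocks re-attacks until the montage completes.
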(event `self.ReceiveBeginPlay`
  ;[1 1 1] Monster Sensing System
  (`KismetSystemLibrary.K2_SetTimerDelegate` (delegate `StopSeeingPlayer`) 0.8 true))

(event `StopSeeingPlayer`
  ;[1 1 1] Monster Sensing System
  (`BlackboardComponent.SetValueAsBool` (`AIBlueprintHelperLibrary.GetBlackboard` (`AIBlueprintHelperLibrary.GetAIController` self)) "seeingPlayer" false)
  (`KismetSystemLibrary.Delay` 1.0)
  (if (not (`BlackboardComponent.GetValueAsBool` (`AIBlueprintHelperLibrary.GetBlackboard` (`AIBlueprintHelperLibrary.GetAIController` self)) "seeingPlayer"))
    (bind _chasingmusic (`self.ChasingMusic`)
      (:`then`
        (`AudioComponent.FadeOut` _chasingmusic 3.0 0.0 "Linear"))
      (:`else`))))

(event `self.PawnSensing.OnSeePawn`
  (params (Pawn :type "Pawn Object Reference"))
  ;[1 1 1] Monster Sensing System
  (if (`self.ActorHasTag` Pawn "Player")
    (`BlackboardComponent.SetValueAsBool` (`AIBlueprintHelperLibrary.GetBlackboard` (`AIBlueprintHelperLibrary.GetAIController` self)) "seeingPlayer" true)
    (`self.ChasingMusic`
      (:`then`)
      (:`else`
        (bind _returnvalue (`GameplayStatics.SpawnSound2D` "/Game/Sounds/ChasingSound.ChasingSound" 1.0 1.0 0.0 null))
        (bind _output_get (set `self.ChasingMusic` _returnvalue))
        (`AudioComponent.FadeIn` _output_get 3.0 1.0 0.0 "Linear")))))

(event `AttackPlayer`
  (bind _attacktracepoint (`self.AttackTracePoint`))
  (bind _returnvalue (`SceneComponent.K2_GetComponentLocation` _attacktracepoint))
  ;[1 1 1] Monster Attack System
  (if (not (`self.Attacking`))
    (set `self.Attacking` true)
    (`|PlayMontage` (`self.Mesh`) "/Game/Enemy/Zombie_Attack_Montage.Zombie_Attack_Montage"
      (:`then`
        (bind (_outhit _returnvalue_2) (`KismetSystemLibrary.SphereTraceSingleForObjects` _returnvalue (+ _returnvalue (* (`KismetMathLibrary.GetForwardVector` (`SceneComponent.K2_GetComponentRotation` _attacktracepoint)) 70.0)) 25.0 (`|MakeArray` "ObjectTypeQuery3" :!type "EObjectTypeQuery Enum")))
        (if _returnvalue_2
          (`GameplayStatics.ApplyDamage` (`.HitActor` (`GameplayStatics.BreakHitResult` _outhit)) 10.0)))
      (:`OnCompleted`
        (set `self.Attacking` false)))))

(fn `UserConstructionScript`)