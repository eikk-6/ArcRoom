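; BP_Drawer is an interactable drawer that the player can get inside and out of.
; Its Interact event toggles an Inside flag and teleports player character 0 to the REFInside or REFOutside reference, matching location and rotation.
; Each toggle also snaps the Door to a different fixed relative rotation, with no animation.
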(event `/Game/BluePrint/BPI_Interaction.Interact`
  (bind (_returnvalue_location _returnvalue_rotation) (`KismetMathLibrary.BreakTransform` (`SceneComponent.K2_GetComponentToWorld` (`self.REFOutside`))))
  (bind (_returnvalue_location_2 _returnvalue_rotation_2) (`KismetMathLibrary.BreakTransform` (`SceneComponent.K2_GetComponentToWorld` (`self.REFInside`))))
  ;[1 1 1] Drawer System
  (if (not (`self.Inside`))
    (set `self.Inside` true)
    (`self.K2_SetActorTransform` (`GameplayStatics.GetPlayerCharacter` 0) (`KismetMathLibrary.MakeTransform` _returnvalue_location_2 _returnvalue_rotation_2) false false)
    (`SceneComponent.K2_SetRelativeRotation` (`self.Door`) (struct :`Yaw` -90.0) false false)
    (else
      (set `self.Inside` false)
      (`self.K2_SetActorTransform` (`GameplayStatics.GetPlayerCharacter` 0) (`KismetMathLibrary.MakeTransform` _returnvalue_location _returnvalue_rotation) false false)
      (`SceneComponent.K2_SetRelativeRotation` (`self.Door`) (struct :`Yaw` 20.0) false false))))

(fn `UserConstructionScript`)