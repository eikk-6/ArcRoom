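; BP_ExitDoor is an exit door that opens on interaction once all collectables are gathered.
; Interact reads CollectablesLeft from BP_ThirdPersonGameMode and, at zero, plays a timeline that swings the Door's yaw open by a quarter turn.
; Otherwise it creates a WB_NotCollectable widget and adds it to the viewport.
; The OpenDoor event is empty.
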(event `/Game/BluePrint/BPI_Interaction.Interact`
  ;[1 1 1] Exit Door Open System
  (bind _asbp_third_person_game_mode (cast `/Game/ThirdPerson/Blueprints/BP_ThirdPersonGameMode` (`GameplayStatics.GetGameMode`)))
  (if (== (`/Game/ThirdPerson/Blueprints/BP_ThirdPersonGameMode.CollectablesLeft` _asbp_third_person_game_mode) 0)
    (bind (_direction _doorfloat) (`Timeline|OpenDoor Timeline`)
      (:`Update`
        (`SceneComponent.K2_SetRelativeRotation` (`self.Door`) (`KismetMathLibrary.MakeRotator` 0.0 0.0 (`KismetMathLibrary.Lerp` 0.0 90.0 _doorfloat)) false false)))
    (else
      (bind _returnvalue (`|CreateWidget` "/Game/UI/WB_NotCollectable.WB_NotCollectable_C"))
      (`UserWidget.AddToViewport` _returnvalue 0))))

(event `OpenDoor`)

(fn `UserConstructionScript`)